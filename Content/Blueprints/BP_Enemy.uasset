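; BP_Enemy is an enemy actor that flies in a straight line and ends the game when it hits the player.
; On spawn, a random roll against TraceRate either aims it once at BP_Player's position, destroying itself if none exists, or keeps its forward vector.
; Tick moves it by MoveSpeed without sweeping.
; Overlapping the player destroys both, spawns an explosion, shows the game-over widget and cursor, and pauses the game.
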(event EventTick
  (params (DeltaSeconds :type Float%20%28single-precision%29))
  ;[1 1 1] Enemey 이동속도
  (Transformation|SetActorLocation (+ (Transformation|GetActorLocation) (* (* (Variables|Default|GetDirection) (Variables|Default|GetMoveSpeed)) DeltaSeconds)) false false))

(event Collision|EventActorBeginOverlap
  (params (OtherActor :type Actor%20Object%20Reference))
  ;[1 1 1] 플레이어와 충돌감지
  (bind _asbp_player (Utilities|Casting|CastToBP_Player OtherActor))
  (Actor|DestroyActor _asbp_player)
  (Effects|SpawnEmitteratLocation "/Game/StarterContent/Particles/P_Explosion.P_Explosion" (Transformation|GetActorLocation))
  (bind _returnvalue (Game|ConstructObjectfromClass "/Game/UI/WBP_GameOverWidget.WBP_GameOverWidget_C"))
  (UserInterface|Viewport|AddtoViewport _returnvalue 0)
  (Variables|/Script/Engine.PlayerController|SetbShowMouseCursor (Game|GetPlayerController 0) true)
  (Game|SetGamePaused true)
  (Actor|DestroyActor))

(event EventBeginPlay
  ;[1 1 1] 생성시 랜덤으로 플레이어를 추적하는 로직
  (if (<= (Math|Random|RandomFloatinRange 0.0 1.0) (Variables|Default|GetTraceRate))
    (bind _returnvalue (Actor|GetActorOfClass "/Game/Blueprints/BP_Player.BP_Player_C"))
    (Utilities|IsValid _returnvalue
      (:Is%20Valid
        (bind _output_get (Variables|Default|SetDirection (Math|Vector|Normalize (- (Transformation|GetActorLocation _returnvalue) (Transformation|GetActorLocation)))))
        (Transformation|SetActorRotation (Math|Rotator|MakeRotfromXZ _output_get (Transformation|GetActorUpVector))))
      (:Is%20Not%20Valid
        (Actor|DestroyActor)))
    (else
      (Variables|Default|SetDirection (Transformation|GetActorForwardVector)))))

(fn ConstructionScript)