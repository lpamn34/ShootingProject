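; BP_GameModBase is a game mode Blueprint that shows the main HUD and tracks the current and persistent best score.
; On BeginPlay it creates WBP_MainWidget and loads BestScore from a BP_SaveScore save slot, if one exists.
; AddScore accumulates points into CurrentScore and, whenever that beats BestScore, immediately writes the new record through a fresh BP_SaveScore object.
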(event EventBeginPlay
  (bind _returnvalue (UserInterface|CreateWidget "/Game/UI/WBP_MainWidget.WBP_MainWidget_C"))
  (UserInterface|Viewport|AddtoViewport _returnvalue 0)
  (bind _bast_score (CallFunction|LodeScoreData))
  (Variables|Default|SetBestScore _bast_score))

(fn ConstructionScript)

(fn AddScore
  (params (Point :type Integer))
  ;[1 1 1] 최고점수 갱신로직
  (bind _output_get (Variables|Default|SetCurrentScore (+ Point (Variables|Default|GetCurrentScore))))
  (if (> _output_get (Variables|Default|GetBestScore))
    (bind _output_get_2 (Variables|Default|SetBestScore _output_get))
    (CallFunction|SaveScoreData _output_get_2)))

(fn SaveScoreData
  (params (Save%20Value :type Integer))
  (bind _returnvalue (SaveGame|CreateSaveGameObject "/Game/Blueprints/BP_SaveScore.BP_SaveScore_C"))
  (bind _output_get (Variables|Default|SetSave%20Instance _returnvalue))
  (Variables|/Game/Blueprints/BP_SaveScore.BP_SaveScore_C|SetScoreData _output_get Save%20Value)
  (SaveGame|SaveGametoSlot _output_get "BastScoreData"))

(fn LodeScoreData
  (bind _returnvalue (SaveGame|DoesSaveGameExist "BastScoreData"))
  (if _returnvalue
    (bind _returnvalue_2 (SaveGame|LoadGamefromSlot "BastScoreData"))
    (bind _asbp_save_score (Utilities|Casting|CastToBP_SaveScore _returnvalue_2))
    (return (Variables|/Game/Blueprints/BP_SaveScore.BP_SaveScore_C|GetScoreData _asbp_save_score))))