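; BP_Player is the player-controlled actor that moves in the Y-Z plane and fires bullets.
; Enhanced Input actions from IMC_PlayerInput, registered on BeginPlay, store the horizontal and vertical axis values.
; Tick normalizes them to even out diagonal speed, then offsets the location by MoveSpeed and delta time without sweeping.
; Pressing fire spawns a BP_Bullet at the FierPositon component's transform.
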(event Input|EnhancedActionEvents|EnhancedInputActionIA_Horizontal
  (params (ActionValue :type Float%20%28double-precision%29) (ElapsedSeconds :type Float%20%28double-precision%29) (TriggeredSeconds :type Float%20%28double-precision%29) (InputAction :type Input%20Action%20Object%20Reference :default "/Game/Inputs/IA_Horizontal.IA_Horizontal"))
  ;[1 1 1] 플레이어 조작
  (:Triggered
    (Variables|Default|SetHorizontal ActionValue))
  (:Completed
    (Variables|Default|SetHorizontal ActionValue)))

(event Input|EnhancedActionEvents|EnhancedInputActionIA_Vertical
  (params (ActionValue :type Float%20%28double-precision%29) (ElapsedSeconds :type Float%20%28double-precision%29) (TriggeredSeconds :type Float%20%28double-precision%29) (InputAction :type Input%20Action%20Object%20Reference :default "/Game/Inputs/IA_Vertical.IA_Vertical"))
  ;[1 1 1] 플레이어 조작
  (:Triggered
    (Variables|Default|SetVertical ActionValue))
  (:Completed
    (Variables|Default|SetVertical ActionValue)))

(event Input|EnhancedActionEvents|EnhancedInputActionIA_Fire
  (params (ActionValue :type Boolean) (ElapsedSeconds :type Float%20%28double-precision%29) (TriggeredSeconds :type Float%20%28double-precision%29) (InputAction :type Input%20Action%20Object%20Reference :default "/Game/Inputs/IA_Fire.IA_Fire"))
  ;[1 1 1] 총알 생성
  (:Started
    (Game|SpawnActorfromClass "/Game/Blueprints/BP_Bullet.BP_Bullet_C" (Transformation|GetWorldTransform (Variables|Default|GetFier%20Positon)) "AlwaysSpawn" "MultiplyWithRoot" 0 0)))

(event EventBeginPlay
  (Input|AddMappingContext (PlayerController|LocalPlayerSubsystems|GetEnhancedInputLocalPlayerSubsystem (Game|GetPlayerController 0)) "/Game/Inputs/IMC_PlayerInput.IMC_PlayerInput" 0 "(bIgnoreAllPressedKeysUntilRelease=True,bForceImmediately=False,bNotifyUserSettings=False)"))

(event EventTick
  (params (DeltaSeconds :type Float%20%28single-precision%29))
  ;[1 1 1] 플레이어의 속도 계산
  ;;[1 1 1] 델타타임 보정
  (Transformation|SetActorLocation (+ (Transformation|GetActorLocation) (* (* (Math|Vector|Normalize (Math|Vector|MakeVector 0.0 (Variables|Default|GetHorizontal) (Variables|Default|GetVertical))) (Variables|Default|GetMoveSpeed)) DeltaSeconds)) false false))

(fn ConstructionScript)